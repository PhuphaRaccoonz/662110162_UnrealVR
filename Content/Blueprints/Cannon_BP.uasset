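; Cannon actor that runs a one-shot firing sequence automatically on BeginPlay.
; A timeline first rotates the lever pivot from its initial rotation to an end rotation, then a second timeline swings the cannon pivot the same way.
; When the cannon finishes rotating, it spawns an enlarged projectile at the shooting point's location and rotation.
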(event `self.ReceiveBeginPlay`
  (bind (_returnvalue_location _returnvalue_rotation) (`KismetMathLibrary.BreakTransform` (`SceneComponent.K2_GetComponentToWorld` (`self.Shooting Point`))))
  (set `self.Lever First Rotation` (`SceneComponent.RelativeRotation` (`self.Lever Rotating Point`)))
  (set `self.Cannon First Rotation` (`SceneComponent.RelativeRotation` (`self.Cannon Rotating Point`)))
  (bind (_direction _time) (`Timeline|Pull Lever` :!via `PlayFromStart`)
    (:`Update`
      (`SceneComponent.K2_SetRelativeRotation` (`self.Lever Rotating Point`) (`KismetMathLibrary.RLerp` (`self.Lever First Rotation`) (`self.Lever End Rotation`) _time) false false))
    (:`Finished`
      (bind (_direction_2 _time_2) (`Timeline|Rotate Cannon` :!via `PlayFromStart`)
        (:`Update`
          (`SceneComponent.K2_SetRelativeRotation` (`self.Cannon Rotating Point`) (`KismetMathLibrary.RLerp` (`self.Cannon First Rotation`) (`self.Cannon End Rotation`) _time_2) false false))
        (:`Finished`
          (`|SpawnActorFromClass` "/Game/VRTemplate/Blueprints/Projectile.Projectile_C" (`KismetMathLibrary.MakeTransform` _returnvalue_location _returnvalue_rotation (10.0 10.0 10.0)) "Undefined" "MultiplyWithRoot" null null))))))

(fn `UserConstructionScript`)